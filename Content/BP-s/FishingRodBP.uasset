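; FishingRodBP is a fishing rod pickup that the third-person character collects by pressing F.
; Its Trigger overlap enables input for player controller 0 and end overlap disables it, with no filter on the overlapping actor.
; On F, it casts the begin-overlap actor to BP_ThirdPersonCharacter, adds Collected to that character's HasFishingRod, then destroys itself.
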(event `self.Trigger.OnComponentBeginOverlap`
  (params (OverlappedComponent :type "PrimitiveComponent Object Reference") (OtherActor :type "Actor Object Reference") (OtherComp :type "PrimitiveComponent Object Reference") (OtherBodyIndex :type Integer) (bFromSweep :type Boolean) (SweepResult :type "HitResult Structure (by ref)"))
  (`self.EnableInput` (`GameplayStatics.GetPlayerController` 0)))

(event `Key|F`
  (params (Key :type "Key Structure"))
  (:`Pressed`
    (bind _asbp_third_person_character (cast `/Game/ThirdPerson/Blueprints/BP_ThirdPersonCharacter` (stale `self.Trigger.OnComponentBeginOverlap` OtherActor)))
    (set `/Game/ThirdPerson/Blueprints/BP_ThirdPersonCharacter.HasFishingRod` (+ (`/Game/ThirdPerson/Blueprints/BP_ThirdPersonCharacter.HasFishingRod` _asbp_third_person_character) (`self.Collected`)) _asbp_third_person_character)
    (`self.K2_DestroyActor`)))

(event `self.Trigger.OnComponentEndOverlap`
  (params (OverlappedComponent :type "PrimitiveComponent Object Reference") (OtherActor :type "Actor Object Reference") (OtherComp :type "PrimitiveComponent Object Reference") (OtherBodyIndex :type Integer))
  (`self.DisableInput` (`GameplayStatics.GetPlayerController` 0)))

(fn `UserConstructionScript`)